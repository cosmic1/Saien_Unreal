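; BP_TimeDialtionAdjustment is a component that gives its owning actor its own time dilation.
; On BeginPlay it copies its CustomTimeDilation value onto the owner, and Tick does nothing.
; An unconnected branch, which never runs, would cap the static mesh's physics linear velocity at a fixed speed and print the owner's velocity.
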(event EventBeginPlay
  (Variables|/Script/Engine.Actor|SetCustomTimeDilation (Components|GetOwner) (Variables|Default|GetCustom%20Time%20Dilation)))

(event EventTick
  (params (DeltaSeconds :type Float%20%28single-precision%29)))